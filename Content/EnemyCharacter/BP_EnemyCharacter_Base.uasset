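; Base enemy character Blueprint that implements the death dissolve effect.
; On OnEnemyDied it pauses animation, disables capsule collision and async-loads the passed Niagara system, attaching it to the mesh with particle color taken from the material's DissolveEdgeColor.
; After that load, a timeline rate-scaled by TotalDissolveTime drives DissolveAmount on the body and equipped weapon materials, then destroys both actors when finished.
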(event EventBeginPlay)

(event Collision|EventActorBeginOverlap
  (params (OtherActor :type Actor%20Object%20Reference)))

(event EventTick
  (params (DeltaSeconds :type Float%20%28single-precision%29)))

(event EventOnEnemyDied
  (params (DissolveNiagaraSystem :type Niagara%20System%20Soft%20Object%20Reference))
  (bind _enemycombatcomponent (Variables|Default|GetEnemyCombatComponent))
  (bind _enemycombatcomponent_2 (Variables|Default|GetEnemyCombatComponent))
  (bind _mesh (Variables|Character|GetMesh))
  (bind _returnvalue (Class|PawnCombatComponent|GetCharacterCurrentEquippedWeapon _enemycombatcomponent))
  (bind _returnvalue_2 (Class|PawnCombatComponent|GetCharacterCurrentEquippedWeapon _enemycombatcomponent_2))
  (Utilities|FlowControl|Sequence
    (:then_0
      (Variables|/Script/Engine.SkeletalMeshComponent|SetbPauseAnims (Variables|Character|GetMesh) true)
      (Collision|SetCollisionEnabled (Variables|Default|GetCapsuleComponent) "NoCollision"))
    (:then_1
      (bind _object (Utilities|AsyncLoadAsset DissolveNiagaraSystem)
        (:Completed
          (bind _asniagara_system (Utilities|Casting|CastToNiagaraSystem _object))
          (bind _returnvalue_3 (Niagara|SpawnSystemAttached _asniagara_system (Variables|Character|GetMesh) "None" "0, 0, 0" "0, 0, 0" "KeepRelativeOffset" true))
          ;[1 1 1] 머티리얼 인스턴스에서 색상값 받아와서 나이아가라에도 설정
          (bind _returnvalue_4 (Rendering|Material|CreateDynamicMaterialInstance _mesh 0 (Rendering|Material|GetMaterial _mesh 0) "None" :!class /Script/Engine.PrimitiveComponent))
          (bind _returnvalue_5 (Rendering|Material|GetVectorParameterValue _returnvalue_4 "DissolveEdgeColor" :!class /Script/Engine.MaterialInstanceDynamic))
          (Niagara|SetNiagaraVariable(LinearColor) _returnvalue_3 "DissolveParticleColor" _returnvalue_5)
          (Components|Timeline|SetPlayRate (Variables|Default|GetDissolveTimeline) (/ 1.0 (Variables|Default|GetTotalDissolveTime)))
          (bind _normalizedfloattrack (Timeline|DissolveTimeline PlayFromStart)
            (:Update
              (Rendering|Material|SetScalarParameterValueonMaterials (Variables|Character|GetMesh) "DissolveAmount" _normalizedfloattrack)
              (Utilities|IsValid _returnvalue_2
                (:Is%20Valid
                  (Rendering|Material|SetScalarParameterValueonMaterials (Variables|/Script/Warrior.WarriorWeaponBase|GetWeaponMesh _returnvalue_2) "DissolveAmount" _normalizedfloattrack))))
            (:Finished
              (Utilities|IsValid _returnvalue
                (:Is%20Valid
                  (Actor|DestroyActor _returnvalue))
                (:Is%20Not%20Valid
                  _))
              (Actor|DestroyActor))))))))

(fn ConstructionScript)